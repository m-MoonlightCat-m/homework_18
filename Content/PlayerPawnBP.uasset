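; PlayerPawnBP is the player pawn Blueprint that sets up the score display and opens the pause menu.
; On BeginPlay it creates a ScoreBlock widget and adds it to the viewport.
; Pressing P pauses the game, shows the mouse cursor, creates a Menu widget stored in WBPMenu, and switches input to UI-only focused on that menu.
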(event `self.ReceiveBeginPlay`
  (bind _returnvalue (`|CreateWidget` "/Game/HUD/ScoreBlock.ScoreBlock_C"))
  (`UserWidget.AddToViewport` _returnvalue 0))

(event `Key|P` :paused true
  (params (Key :type "Key Structure"))
  (:`Pressed`
    (`GameplayStatics.SetGamePaused` true)
    (set `PlayerController.bShowMouseCursor` true (`GameplayStatics.GetPlayerController` 0))
    (bind _returnvalue (`|CreateWidget` "/Game/HUD/Menu.Menu_C"))
    (bind _output_get (set `self.WBP_Menu` _returnvalue))
    (`UserWidget.AddToViewport` _output_get 0)
    (`WidgetBlueprintLibrary.SetInputMode_UIOnlyEx` (`GameplayStatics.GetPlayerController` 0) (`self.WBP_Menu`))))

(fn `UserConstructionScript`)